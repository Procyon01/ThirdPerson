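; ProxLight is a spotlight actor that the player can toggle on and off with F while standing within its proximity trigger.
; Overlapping ProxTrigger enables input for player controller 0 and leaving disables it, with both events flipping the HintText prompt's visibility.
; The construction script applies the LightColor and VisibilitySetting variables to the SpotLight, setting its color and initial on/off state.
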(event `Key|F`
  (params (Key :type "Key Structure"))
  ;[1 1 1] press F to toggle light when in proximity
  (:`Pressed`
    (`SceneComponent.ToggleVisibility` (`self.SpotLight`) false)))

(event `self.ProxTrigger.OnComponentBeginOverlap`
  (params (OverlappedComponent :type "PrimitiveComponent Object Reference") (OtherActor :type "Actor Object Reference") (OtherComp :type "PrimitiveComponent Object Reference") (OtherBodyIndex :type Integer) (bFromSweep :type Boolean) (SweepResult :type "HitResult Structure (by ref)"))
  ;[1 1 1] When overlapping trigger, enable input/show prompt. When leaving, disable input and remove prompt
  (`self.EnableInput` (`GameplayStatics.GetPlayerController` 0))
  (`SceneComponent.ToggleVisibility` (`self.HintText`) false :!label _label))

(event `self.ProxTrigger.OnComponentEndOverlap`
  (params (OverlappedComponent :type "PrimitiveComponent Object Reference") (OtherActor :type "Actor Object Reference") (OtherComp :type "PrimitiveComponent Object Reference") (OtherBodyIndex :type Integer))
  ;[1 1 1] When overlapping trigger, enable input/show prompt. When leaving, disable input and remove prompt
  (`self.DisableInput` (`GameplayStatics.GetPlayerController` 0))
  (goto _label))

(fn `UserConstructionScript`
  (bind _spotlight (`self.SpotLight`))
  (`LightComponent.SetLightColor` _spotlight (`self.LightColor`) true)
  (`SceneComponent.SetVisibility` _spotlight (`self.Visibility Setting`) false))